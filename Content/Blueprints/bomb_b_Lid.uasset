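; Bomb lid actor that slides away and disappears once the panel removal step signals a drop.
; Each Tick it searches for all PanelRemoval actors and reads the Drop flag on the first one found.
; While Drop is set, it moves along its local Z axis by a fixed per-frame offset, independent of delta time, and counts down a short timer before destroying itself.
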(event `self.ReceiveBeginPlay`
  (set `self.DeathTimer` 5.0))

(event `self.ReceiveTick`
  (params (DeltaSeconds :type "Float (single-precision)"))
  (bind _outactors (`GameplayStatics.GetAllActorsOfClass` "/Game/Bomb_Parts/PanelRemoval.PanelRemoval_C"))
  (if (`/Game/Bomb_Parts/PanelRemoval.Drop` (`KismetArrayLibrary.Array_Get` _outactors))
    (`self.K2_AddActorLocalOffset` (0.0 0.0 1.0))
    (set `self.DeathTimer` (- (`self.DeathTimer`) DeltaSeconds))
    (if (<= (`self.DeathTimer`) 0.0)
      (`self.K2_DestroyActor`))))

(fn `UserConstructionScript`)