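; Screw actor that spins loose while another actor overlaps it, then falls out.
; Begin and end overlap toggle an unscrewing flag, which lets Tick rotate the mesh and drain an unscrew timer.
; Once that timer runs out, Tick moves the mesh down along its local axis until a second timer marks it dead and stops the motion, without destroying the actor.
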(event `self.ReceiveBeginPlay`
  (set `self.UnscrewLife` 3.0)
  (set `self.DeathTimer` 2.0))

(event `self.ReceiveActorBeginOverlap`
  (params (OtherActor :type "Actor Object Reference"))
  (set `self.Unscrewing` true))

(event `self.ReceiveActorEndOverlap`
  (params (OtherActor :type "Actor Object Reference"))
  (set `self.Unscrewing` false))

(event `self.ReceiveTick`
  (params (DeltaSeconds :type "Float (single-precision)"))
  (bind _unscrewing (`self.Unscrewing`))
  (bind _returnvalue (>= (`self.UnscrewLife`) 0.0))
  (if (or _returnvalue (and _returnvalue _unscrewing))
    (if _unscrewing
      (`SceneComponent.K2_AddLocalRotation` (`self.StaticMesh`) (struct :`Yaw` 5.0) false false)
      (set `self.UnscrewLife` (- (`self.UnscrewLife`) DeltaSeconds)))
    (elif _returnvalue
      _
      (elif (not (`self.Dead`))
        (`SceneComponent.K2_AddLocalOffset` (`self.StaticMesh`) (0.0 0.0 -2.2) false false)
        (set `self.DeathTimer` (- (`self.DeathTimer`) DeltaSeconds))
        (if (<= (`self.DeathTimer`) 0.0)
          (set `self.Dead` true))))))

(fn `UserConstructionScript`)