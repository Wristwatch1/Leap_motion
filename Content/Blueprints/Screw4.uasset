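; Screw4 is a screw actor that unscrews and then drops as other actors overlap it.
; Each begin-overlap event rotates the static mesh a step and reduces UnscrewLife by Tick's DeltaSeconds, so progress advances per overlap rather than continuously.
; Once that life is below zero, overlaps shift the mesh down its local Z and reduce DeathTimer until the Dead flag stops movement.
; Tick itself runs no logic.
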(event `self.ReceiveBeginPlay`
  (set `self.UnscrewLife` 3.0)
  (set `self.DeathTimer` 2.0))

(event `self.ReceiveActorBeginOverlap`
  (params (OtherActor :type "Actor Object Reference"))
  (if (>= (`self.UnscrewLife`) 0.0)
    (`SceneComponent.K2_AddLocalRotation` (`self.StaticMesh`) (struct :`Yaw` 5.0) false false)
    (set `self.UnscrewLife` (- (`self.UnscrewLife`) (stale `self.ReceiveTick` DeltaSeconds)))
    (elif (not (`self.Dead`))
      (`SceneComponent.K2_AddLocalOffset` (`self.StaticMesh`) (0.0 0.0 -1.0) false false)
      (set `self.DeathTimer` (- (`self.DeathTimer`) (stale `self.ReceiveTick` DeltaSeconds)))
      (if (<= (`self.DeathTimer`) 0.0)
        (set `self.Dead` true)))))

(event `self.ReceiveTick`
  (params (DeltaSeconds :type "Float (single-precision)")))

(fn `UserConstructionScript`)